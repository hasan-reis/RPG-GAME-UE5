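; Animation notify that toggles combat mode on the owning actor at a point in an animation, such as drawing or sheathing a weapon.
; It fetches the owner's combat component and, if a main weapon exists, attaches it to either the hand socket or its stowed socket based on the EnableComponent flag.
; It then passes the same flag to the component's combat-enabled state.
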(fn ReceivedNotify
  (params (MeshComp :type Skeletal%20Mesh%20Component%20Object%20Reference) (Animation :type Anim%20Sequence%20Base%20Object%20Reference) (EventReference :type Anim%20Notify%20Event%20Reference%20Structure%20%28by%20ref%29))
  (bind _returnvalue (Components|GetOwner MeshComp))
  (bind _returnvalue_2 (Actor|GetComponentbyClass _returnvalue "/Game/CombatSystem/Blueprints/Components/BP_CombatComponent_BP.BP_CombatComponent_BP_C"))
  (bind _mainweapon (Default|GetMainWeapon _returnvalue_2))
  (Utilities|IsValid _mainweapon
    (:Is%20Valid
      (Default|AttachActor _mainweapon (select (Variables|Default|GetbEnableComponent?) (Variables|/Game/CombatSystem/Blueprints/Actors/BP_BaseWeapon.BP_BaseWeapon_C|GetHandSocketName _mainweapon) (Variables|/Game/CombatSystem/Blueprints/Actors/BP_BaseEquippable.BP_BaseEquippable_C|GetAttachSocketName _mainweapon)))
      (Default|SetCombatEnabled _returnvalue_2 (Variables|Default|GetbEnableComponent?))
      (return true))
    (:Is%20Not%20Valid
      (return false))))