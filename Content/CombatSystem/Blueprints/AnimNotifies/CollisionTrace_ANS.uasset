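; Anim notify state that opens and closes the melee hit window of the owning actor's main weapon during an animation.
; On begin, it gets the combat component from the mesh owner, fetches the main weapon and enables collision on that weapon's collision component.
; On end, it disables that collision, and both events return false when no valid main weapon exists.
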(fn ReceivedNotifyBegin
  (params (MeshComp :type Skeletal%20Mesh%20Component%20Object%20Reference) (Animation :type Anim%20Sequence%20Base%20Object%20Reference) (TotalDuration :type Float%20%28single-precision%29) (EventReference :type Anim%20Notify%20Event%20Reference%20Structure%20%28by%20ref%29))
  (bind _returnvalue (Components|GetOwner MeshComp))
  (bind _returnvalue_2 (Actor|GetComponentbyClass _returnvalue "/Game/CombatSystem/Blueprints/Components/BP_CombatComponent_BP.BP_CombatComponent_BP_C"))
  (bind _mainweapon (Default|GetMainWeapon _returnvalue_2))
  (Utilities|IsValid _mainweapon
    (:Is%20Valid
      (Default|EnableCollision (Variables|/Game/CombatSystem/Blueprints/Actors/BP_BaseWeapon.BP_BaseWeapon_C|GetMainWeaponCollisionComponent _mainweapon))
      (return true))
    (:Is%20Not%20Valid
      (return false))))

(fn ReceivedNotifyEnd
  (params (MeshComp :type Skeletal%20Mesh%20Component%20Object%20Reference) (Animation :type Anim%20Sequence%20Base%20Object%20Reference) (EventReference :type Anim%20Notify%20Event%20Reference%20Structure%20%28by%20ref%29))
  (bind _returnvalue (Components|GetOwner MeshComp))
  (bind _returnvalue_2 (Actor|GetComponentbyClass _returnvalue "/Game/CombatSystem/Blueprints/Components/BP_CombatComponent_BP.BP_CombatComponent_BP_C"))
  (bind _mainweapon (Default|GetMainWeapon _returnvalue_2))
  (Utilities|IsValid _mainweapon
    (:Is%20Valid
      (Default|DisableCollision (Variables|/Game/CombatSystem/Blueprints/Actors/BP_BaseWeapon.BP_BaseWeapon_C|GetMainWeaponCollisionComponent _mainweapon))
      (return true))
    (:Is%20Not%20Valid
      (return false))))