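; Actor component that stores a character's stats for the combat system as base and current values.
; Two maps keyed by stat drive it: BaseStats holds base and max values, and CurrentStats holds live values.
; InitializeStats copies each base value into the current map.
; ModifyCurrentStatValue adds a delta and clamps the result between zero and that stat's max, while getters expose current, base and max values.
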(event EventBeginPlay)

(event EventTick
  (params (DeltaSeconds :type Float%20%28single-precision%29)))

(fn SetCurrentStatValue
  (params (Stat :type E_Stats%20Enum :default "NewEnumerator0") (Value :type Float%20%28double-precision%29))
  (Utilities|Map|Add (Variables|BaseStats|GetCurrentStats) Stat Value))

(fn GetCurrentStatValue
  (params (Key :type E_Stats%20Enum%20%28by%20ref%29 :default "NewEnumerator0"))
  (return (.Value (Utilities|Map|Find (Variables|BaseStats|GetCurrentStats) Key))))

(fn InitializeStats
  (bind _keys (Utilities|Map|Keys (Variables|Default|GetBaseStats)))
  (for _array_element _keys
    (CallFunction|SetCurrentStatValue _array_element (.basevalue (.Value (Utilities|Map|Find (Variables|Default|GetBaseStats) _array_element))))))

(fn ModifyCurrentStatValue
  (params (Stat :type E_Stats%20Enum :default "NewEnumerator0") (Value :type Float%20%28double-precision%29))
  (if (!= 0.0 Value)
    (bind _output_get (LocalVariables|SetL_Value (+ Value (CallFunction|GetCurrentStatValue Stat))))
    (bind _output_get_2 (LocalVariables|SetL_Value (Math|Float|Clamp(Float) _output_get 0.0 (BaseStats|GetMaxStatValue Stat))))
    (CallFunction|SetCurrentStatValue Stat _output_get_2)))

(fn GetBaseStatValue
  (params (Key :type E_Stats%20Enum%20%28by%20ref%29 :default "NewEnumerator0"))
  (return (.basevalue (.Value (Utilities|Map|Find (Variables|Default|GetBaseStats) Key)))))

(fn GetMaxStatValue
  (params (Key :type E_Stats%20Enum%20%28by%20ref%29 :default "NewEnumerator0"))
  (return (.maxvalue (.Value (Utilities|Map|Find (Variables|Default|GetBaseStats) Key)))))