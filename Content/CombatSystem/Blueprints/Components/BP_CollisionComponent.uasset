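; BP_CollisionComponent is a combat component that detects hits along a mesh between two named sockets while collision is enabled.
; Each Tick it runs a multi sphere trace for objects between the sockets, skipping actors on its ignore list.
; Each actor fires OnHit only once per activation, since enabling collision clears the already-hit list.
; External code sets the mesh, toggles collision and reads the last hit.
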(event Custom|EnableCollision
  (CallFunction|ClearHitActor)
  (Variables|Default|SetbIsCollisionEnabled? true))

(event Custom|DisableCollision
  (Variables|Default|SetbIsCollisionEnabled? false))

(event Custom|ClearHitActor
  (Utilities|Array|Clear (Variables|Default|GetAlreadyHitActor)))

(event Custom|CollisionTrace
  (bind _collisionmeshcomponent (Variables|Default|GetCollisionMeshComponent))
  (bind _outhits (Collision|MultiSphereTraceForObjects (Transformation|GetSocketLocation _collisionmeshcomponent (Variables|Initialization|GetStartSocketName)) (Transformation|GetSocketLocation _collisionmeshcomponent (Variables|Initialization|GetEndSocketName)) (Variables|Default|GetRadius) (Variables|Initialization|GetCollision%20Object%20Types) false (Variables|Default|GetActors%20to%20Ignore) (Variables|Initialization|GetDraw%20Debug%20Type)))
  (for _array_element _outhits
    (bind _output_get (Variables|Default|SetLastHit _array_element))
    (if (not (Utilities|Array|ContainsItem (Variables|Default|GetAlreadyHitActor) (.HitActor (Collision|BreakHitResult _output_get))))
      (bind _output_get_2 (Variables|Default|SetHitActor (.HitActor (Collision|BreakHitResult _output_get))))
      (Utilities|Array|Add (Variables|Default|GetAlreadyHitActor) _output_get_2)
      (Default|CallOnHit (Variables|Default|GetLastHit)))))

(event Custom|SetCollisionMesh
  (params (MeshComponent :type Primitive%20Component%20Object%20Reference))
  (Variables|Default|SetCollisionMeshComponent MeshComponent))

(event EventBeginPlay)

(event EventTick
  (params (DeltaSeconds :type Float%20%28single-precision%29))
  (if (Variables|Default|GetbIsCollisionEnabled?)
    (CallFunction|CollisionTrace)))

(fn GetAlreadyHitActors
  (return (Variables|Default|GetAlreadyHitActor)))

(fn IsCollisionEnabled
  (return (Variables|Default|GetbIsCollisionEnabled?)))

(fn GetLastHist
  (return (Variables|Default|GetLastHit)))

(fn GetCollisionMeshComponent
  (return (Variables|Default|GetCollisionMeshComponent)))

(fn AddActortoIgnore
  (params (Inplace :type Actor%20Object%20Reference%20%28by%20ref%29))
  (Utilities|Array|AddUnique (Variables|Default|GetActors%20to%20Ignore) Inplace))

(fn RemoveActortoIgnore
  (params (ActorToRemove :type Actor%20Object%20Reference%20%28by%20ref%29))
  (Utilities|Array|RemoveItem (Variables|Default|GetActors%20to%20Ignore) ActorToRemove))

(fn GetActorstoIgnore
  (return (Variables|Default|GetActors%20to%20Ignore)))