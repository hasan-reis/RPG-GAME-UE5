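; BP_BaseWeapon is the base weapon actor for the combat system, holding damage, combat type and montage sets per character action.
; On equip it attaches to a hand or stowed socket by combat state, registers with the owner's combat component and updates the anim instance's combat type.
; Its collision component hits apply point damage to actors that accept damage via interface message.
; It can also switch its mesh to physics simulation.
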(event OnHit(MainWeaponCollisionComponent)
  (params (HitResult :type Hit%20Result%20Structure))
  (bind _hitactor (Collision|BreakHitResult HitResult))
  (bind _returnvalue (Class|CombatBPI|CanReceiveDamage(Message) _hitactor))
  (if _returnvalue
    (Game|Damage|ApplyPointDamage _hitactor (Variables|Default|GetBase%20Damage) (Transformation|GetActorForwardVector (Components|GetOwner)) HitResult (Game|GetInstigatorController) self)))

(event Custom|SimulateWeaponPhysics
  (bind _newparam (CallFunction|GetItemMesh))
  (Collision|SetCollisionProfileName _newparam "PhysicsActor" true :!class /Script/Engine.PrimitiveComponent)
  (Physics|SetSimulatePhysics _newparam true))

(event EventBeginPlay
  (|CallParentFunction) ; This node is disabled and will not be called.\nDrag off pins to build functionality.
)

(event Collision|EventActorBeginOverlap
  (params (OtherActor :type Actor%20Object%20Reference))
  (|CallParentFunction OtherActor) ; This node is disabled and will not be called.\nDrag off pins to build functionality.
)

(event EventTick
  (params (DeltaSeconds :type Float%20%28single-precision%29))
  (|CallParentFunction DeltaSeconds) ; This node is disabled and will not be called.\nDrag off pins to build functionality.
)

(fn ConstructionScript
  (|CallParentFunction))

(fn OnEquipped
  (|CallParentFunction)
  (Variables|Default|SetCombatComponent (Actor|GetComponentbyClass (Components|GetOwner) "/Game/CombatSystem/Blueprints/Components/BP_CombatComponent_BP.BP_CombatComponent_BP_C"))
  (CallFunction|AttachActor (select (Default|IsCombatEnabled (Variables|Default|GetCombatComponent)) (Variables|Default|GetHandSocketName) (Variables|Default|GetAttachSocketName)))
  (Default|SetMainWeapon (Variables|Default|GetCombatComponent) self)
  (Class|AnimInstanceBPI|UpdateCombatType(Message) (Components|SkeletalMesh|GetAnimInstance (Variables|/Script/Engine.Character|GetMesh (.AsCharacter (Utilities|Casting|CastToCharacter (Components|GetOwner))))) (Variables|Default|GetCombatType))
  (Default|SetCollisionMesh (Variables|Default|GetMainWeaponCollisionComponent) (CallFunction|GetItemMesh))
  (Default|AddActortoIgnore (Variables|Default|GetMainWeaponCollisionComponent) (Components|GetOwner)))

(fn GetActionMontages
  (params (CharacterAction :type E_CharacterAction%20Enum :default "NewEnumerator0"))
  (return (Utilities|Select :Index CharacterAction :NewEnumerator0 0 :NewEnumerator8 0 :NewEnumerator1 (Variables|Montages|GetLightAttackMontages) :NewEnumerator2 (Variables|Montages|GetHeavy%20Attack%20Montages) :NewEnumerator9 (Variables|Montages|GetSprint%20Attack%20%20Montages) :NewEnumerator3 (Variables|Montages|GetCharged%20Attack%20Montages) :NewEnumerator4 (Variables|Montages|GetFalling%20Attack%20Montages) :NewEnumerator5 (Variables|Montages|GetDodgeMontages) :NewEnumerator6 (Utilities|Array|MakeArray (Variables|Montages|GetEnterCombat)) :NewEnumerator7 (Utilities|Array|MakeArray (Variables|Montages|GetExitCombat)))))